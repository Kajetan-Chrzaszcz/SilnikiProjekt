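; BP_Switch is a three-button sequence puzzle that turns on two point lights when the player triggers the buttons in the order 2, 1, 3.
; Overlap triggers check two progress flags, with correct presses changing the button material and disabling that trigger's collision.
; Wrong presses briefly show a false material, and pressing 3 before 1 also resets button 2.
; The lights start dark and return to their saved intensity on success, then the buttons revert to neutral.
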(event OnComponentBeginOverlap(1)
  (params (OverlappedComponent :type Primitive%20Component%20Object%20Reference) (OtherActor :type Actor%20Object%20Reference) (OtherComp :type Primitive%20Component%20Object%20Reference) (OtherBodyIndex :type Integer) (bFromSweep :type Boolean) (SweepResult :type Hit%20Result%20Structure%20%28by%20ref%29))
  (bind _guzik_1 (Variables|Default|GetGuzik%201))
  (Utilities|IsPlayer OtherActor
    (:IsPlayer
      (if (Variables|Default|GetTrue_2)
        (Variables|Default|SetTrue_1 true)
        (CallFunction|AnserTrue (Variables|Default|GetGuzik%201) (Variables|Default|Get1))
        (else
          ;[1 0.2588 0.2588] Wrong Order
          (Utilities|FalseAnserw _guzik_1 _guzik_1))))))

(event OnComponentBeginOverlap(2)
  (params (OverlappedComponent :type Primitive%20Component%20Object%20Reference) (OtherActor :type Actor%20Object%20Reference) (OtherComp :type Primitive%20Component%20Object%20Reference) (OtherBodyIndex :type Integer) (bFromSweep :type Boolean) (SweepResult :type Hit%20Result%20Structure%20%28by%20ref%29))
  (Utilities|IsPlayer OtherActor
    (:IsPlayer
      (Variables|Default|SetTrue_2 true)
      (CallFunction|AnserTrue (Variables|Default|GetGuzik_2) (Variables|Default|Get2)))))

(event OnComponentBeginOverlap(3)
  (params (OverlappedComponent :type Primitive%20Component%20Object%20Reference) (OtherActor :type Actor%20Object%20Reference) (OtherComp :type Primitive%20Component%20Object%20Reference) (OtherBodyIndex :type Integer) (bFromSweep :type Boolean) (SweepResult :type Hit%20Result%20Structure%20%28by%20ref%29))
  (bind _guzik_3 (Variables|Default|GetGuzik_3))
  (bind _guzik_3_2 (Variables|Default|GetGuzik_3))
  (bind _guzik_2 (Variables|Default|GetGuzik_2))
  (Utilities|IsPlayer OtherActor
    (:IsPlayer
      (if (Variables|Default|GetTrue_2)
        (if (Variables|Default|GetTrue_1)
          (CallFunction|AnserTrue (Variables|Default|GetGuzik_3) (Variables|Default|Get3))
          (Rendering|Components|Light|SetIntensity (Variables|Default|GetPointLight_1) (Variables|Default|GetStartPointLightIntensity))
          (Utilities|FlowControl|Delay 1.0)
          (Rendering|Material|SetMaterial (Variables|Default|GetGuzik%201) 0 "/Game/Materials/M_SwitchNeutral.M_SwitchNeutral")
          (else
            ;[1 0.2588 0.2588] Wrong Order
            (Variables|Default|SetTrue_2 false)
            (Utilities|FalseAnserw _guzik_3_2 _guzik_3_2
              (:execute_2
                (Utilities|FalseAnserw _guzik_2 _guzik_2
                  (:execute_2
                    (Collision|SetCollisionEnabled (Variables|Default|Get2) "QueryAndPhysics")))))))
        (else
          ;[1 0.2588 0.2588] Wrong Order
          (Utilities|FalseAnserw _guzik_3 _guzik_3))))))

(event EventBeginPlay
  (bind _pointlight_1 (Variables|Default|GetPointLight_1))
  ;[1 1 1] Light settigs
  (Variables|Default|SetStartPointLightIntensity (Variables|/Script/Engine.LightComponentBase|GetIntensity _pointlight_1))
  (Rendering|Components|Light|SetIntensity _pointlight_1 0.0))

(fn ConstructionScript)

(fn AnserTrue
  (params (Component_1 :type Primitive%20Component%20Object%20Reference) (Collision_1 :type Primitive%20Component%20Object%20Reference))
  (Rendering|Material|SetMaterial Component_1 0 "/Game/Materials/M_SwitchTrue.M_SwitchTrue")
  (Collision|SetCollisionEnabled Collision_1 "NoCollision"))