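; Collectable crystal that spins a fixed yaw step every tick and flies into the player when touched.
; On player overlap it caches its location, scale and light intensity, then plays a timeline.
; The timeline lerps it toward the player pawn's live location while shrinking it to zero and fading its point light on a separate curve.
; The actor destroys itself when finished, with no score or inventory update.
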(event EventBeginPlay)

(event Collision|EventActorBeginOverlap
  (params (OtherActor :type Actor%20Object%20Reference))
  (Utilities|IsPlayer OtherActor
    (:IsPlayer
      (CallFunction|GetStartLerpVariables)
      (bind (_direction _smoothlerpalpha _lightintensityalpha) (Timeline|TL_BlendAlpha Play)
        (:Update
          (CallFunction|ChangeCrystalLoaction _smoothlerpalpha)
          (CallFunction|ChangeCrystalScale3D _smoothlerpalpha)
          (CallFunction|ChangeLightIntensity _lightintensityalpha))
        (:Finished
          (Actor|DestroyActor))))))

(event EventTick
  (params (DeltaSeconds :type Float%20%28single-precision%29))
  (Transformation|SetActorRotation (Math|Rotator|MakeRotator 0.0 0.0 (+ (.yaw (Transformation|GetActorRotation)) 1.0))))

(fn ConstructionScript)

(fn ChangeCrystalLoaction
  (params (Alpha :type Float%20%28single-precision%29))
  (Transformation|SetActorLocation (Math|Vector|Lerp(Vector) (Variables|Default|GetLerpStartLocation) (Transformation|GetActorLocation (Game|Player|GetPlayerPawn 0)) Alpha) false false))

(fn GetStartLerpVariables
  (Variables|Default|SetLerpStartLocation (Transformation|GetActorLocation))
  (Variables|Default|SetLerpStartScale3D (Transformation|GetActorScale3D))
  (Variables|Default|SetLerpStartLightIntensity (Variables|/Script/Engine.LightComponentBase|GetIntensity (Variables|Default|GetPointLight))))

(fn ChangeCrystalScale3D
  (params (Alpha :type Float%20%28single-precision%29))
  (Transformation|SetActorScale3D (Math|Vector|Lerp(Vector) (Variables|Default|GetLerpStartScale3D) "0, 0, 0" Alpha)))

(fn ChangeLightIntensity
  (params (Alpha :type Float%20%28single-precision%29))
  (Rendering|Components|Light|SetIntensity (Variables|Default|GetPointLight) (Math|Float|Lerp (Variables|Default|GetLerpStartLightIntensity) 0.0 Alpha)))